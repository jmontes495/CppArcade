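; Shield_BP is a Space Invaders shield actor that switches its look to a damaged barrier.
; A DestroyedHalfPoint event, guarded by the IsBroken flag so it acts once, sets the Left and Right sprite components to the broken barrier sprite.
; The right half reuses the same sprite, mirrored with a negative X scale.
; The file itself holds no hit detection or health tracking.
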(event `self.ReceiveBeginPlay`
  (set `self.bIsBroken` false))

(event `self.DestroyedHalfPoint`
  (bind _left (`self.Left`))
  (bind _right (`self.Right`))
  (if (not (`self.bIsBroken`))
    (set `self.bIsBroken` true)
    (`PaperSpriteComponent.SetSprite` _left "/Game/SpaceInvaders/Sprites/Invaders/barrier_broken.barrier_broken")
    (`SceneComponent.SetRelativeScale3D` _left (1.0 1.0 1.0))
    (`PaperSpriteComponent.SetSprite` _right "/Game/SpaceInvaders/Sprites/Invaders/barrier_broken.barrier_broken")
    (`SceneComponent.SetRelativeScale3D` _right (-1.0 1.0 1.0))))

(fn `UserConstructionScript`)