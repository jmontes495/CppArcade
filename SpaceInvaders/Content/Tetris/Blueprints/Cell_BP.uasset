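; Cell_BP is a single Tetris board cell that shows its current value as a colored Paper2D sprite.
; SetSprite reads the cell's value and switches the sprite component to the matching block color, using black for empty cells.
; It runs on BeginPlay and again whenever the ChangeSprite event is triggered, so the cell updates only on demand rather than every tick.
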(event `self.ReceiveBeginPlay`
  (`self.SetSprite`))

(event `self.ChangeSprite`
  (`self.SetSprite`))

(fn `SetSprite`
  (bind _returnvalue (`self.GetCurrentCellValue`))
  (switch `ECellValue` _returnvalue
    (:`ECV_Empty`
      (`PaperSpriteComponent.SetSprite` (`self.PaperSprite`) "/Game/Tetris/Sprites/black.black"))
    (:`ECV_Red`
      (`PaperSpriteComponent.SetSprite` (`self.PaperSprite`) "/Game/Tetris/Sprites/red.red"))
    (:`ECV_Orange`
      (`PaperSpriteComponent.SetSprite` (`self.PaperSprite`) "/Game/Tetris/Sprites/orange.orange"))
    (:`ECV_Yellow`
      (`PaperSpriteComponent.SetSprite` (`self.PaperSprite`) "/Game/Tetris/Sprites/yellow.yellow"))
    (:`ECV_Green`
      (`PaperSpriteComponent.SetSprite` (`self.PaperSprite`) "/Game/Tetris/Sprites/green.green"))
    (:`ECV_Cyan`
      (`PaperSpriteComponent.SetSprite` (`self.PaperSprite`) "/Game/Tetris/Sprites/cyan.cyan"))
    (:`ECV_Blue`
      (`PaperSpriteComponent.SetSprite` (`self.PaperSprite`) "/Game/Tetris/Sprites/blue.blue"))
    (:`ECV_Purple`
      (`PaperSpriteComponent.SetSprite` (`self.PaperSprite`) "/Game/Tetris/Sprites/purple.purple"))))

(fn `UserConstructionScript`)